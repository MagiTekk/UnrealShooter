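; M9 pistol pickup with a laser sight for the player's weapon in a shooter.
; The first actor overlap, from any actor, snaps it to the player character mesh's right-hand pistol socket.
; Each tick the laser beam shows only while MainCharacterBP's camera is zoomed in, when a visibility line trace from the laser source sets the beam's end and the impact marker's position, falling back to maximum range on a miss.
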(event `self.ReceiveBeginPlay`)

(event `self.ReceiveActorBeginOverlap`
  (params (OtherActor :type "Actor Object Reference"))
  (`/Engine/EditorBlueprintResources/StandardMacros.DoOnce` false
    (:`Completed`
      (`self.K2_AttachRootComponentTo` (`Character.Mesh` (`GameplayStatics.GetPlayerCharacter` 0)) "hand_rPistolSocket" "SnapToTarget"))))

(event `self.ReceiveTick`
  (params (DeltaSeconds :type "Float (single-precision)"))
  (bind _lasertargetloc (`self.LaserTargetLoc`))
  (bind _lasersource (`self.LaserSource`))
  (bind _returnvalue (`SceneComponent.K2_GetComponentLocation` _lasersource))
  (bind _returnvalue_2 (+ _returnvalue (* (`SceneComponent.GetForwardVector` _lasersource) 5000.0)))
  (bind _asmain_character_bp (cast `/Game/UnrealShooter/Blueprint/Character/MainCharacterBP` (`GameplayStatics.GetPlayerCharacter` 0)))
  (bind _bcamerazoomin (`MainCharacter.bCameraZoomIn` _asmain_character_bp))
  (`SceneComponent.SetVisibility` (`self.LaserBeam`) _bcamerazoomin false)
  (if _bcamerazoomin
    (bind (_outhit _returnvalue_3) (`KismetSystemLibrary.LineTraceSingle` _returnvalue _returnvalue_2 "TraceTypeQuery1"))
    (if _returnvalue_3
      (set `self.LaserTargetLoc` (`.Location` (`GameplayStatics.BreakHitResult` _outhit)))
      (else
        (set `self.LaserTargetLoc` _returnvalue_2)))
    (`ParticleSystemComponent.SetBeamSourcePoint` (`self.LaserBeam`) 0 (`SceneComponent.K2_GetComponentLocation` (`self.LaserSource`)) 0)
    (`ParticleSystemComponent.SetBeamTargetPoint` (`self.LaserBeam`) 0 _lasertargetloc 0)
    (`SceneComponent.K2_SetWorldLocation` (`self.LaserImpact`) (- _lasertargetloc (`SceneComponent.GetForwardVector` (`self.LaserImpact`))) false false)))

(fn `UserConstructionScript`)